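; BP_Meeple is a meeple that awards points and screams once it is knocked away from its starting spot.
; The construction script applies its material and records the mesh's start position.
; A looping timer polls displacement instead of using Tick; past a small threshold it adds Points to BP_GameMode's score and clears itself.
; It then plays a random male or female scream, chosen by UseMaleSounds.
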(event `self.ReceiveBeginPlay`
  (bind _returnvalue (`KismetSystemLibrary.K2_SetTimerDelegate` (delegate `ProcessForPoints`) 0.5 true))
  (set `self.TimerHandle` _returnvalue))

(event `ProcessForPoints`
  (bind _returnvalue (`KismetMathLibrary.RandomIntegerInRange` 1 2))
  (if (>= (`KismetMathLibrary.VSize` (- (`SceneComponent.K2_GetComponentLocation` (`self.StaticMesh`)) (`self.StartPosition`))) 20.0)
    (`/Game/Terror/Core/BP_GameMode.AddScore` (cast `/Game/Terror/Core/BP_GameMode` (`GameplayStatics.GetGameMode`) :!pure true) (`self.Points`))
    (`KismetSystemLibrary.K2_ClearAndInvalidateTimerHandle` (`self.TimerHandle`))
    (if (`self.UseMaleSounds`)
      (`GameplayStatics.PlaySound2D` (select `int` _returnvalue :`0` "/Game/Terror/Audio/A_Scream_Man1.A_Scream_Man1" :`1` "/Game/Terror/Audio/A_Scream_Man2.A_Scream_Man2" :!type "SoundBase Object Reference") 1.0 1.0 0.0 null null)
      (else
        (`GameplayStatics.PlaySound2D` (select `int` _returnvalue :`0` "/Game/Terror/Audio/A_Scream_Lady1.A_Scream_Lady1" :`1` "/Game/Terror/Audio/A_Scream_Lady2.A_Scream_Lady2" :!type "SoundBase Object Reference") 1.0 1.0 0.0 null null)))))

(fn `UserConstructionScript`
  (`PrimitiveComponent.SetMaterial` (`self.StaticMesh`) 0 (`self.Material`))
  (set `self.StartPosition` (`SceneComponent.K2_GetComponentLocation` (`self.StaticMesh`))))