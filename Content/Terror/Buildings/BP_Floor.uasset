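; BP_Floor is a building floor piece that awards points when it is displaced far enough, signalling a collapse.
; The construction script applies the material instance and records the mesh's starting world location.
; A looping one-second timer, used instead of Tick, compares the mesh's displacement against a threshold.
; Once exceeded, it plays the collapse sound, adds points through BP_GameMode and clears the timer, so it scores only once.
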(event `self.ReceiveBeginPlay`
  (bind _returnvalue (`KismetSystemLibrary.K2_SetTimerDelegate` (delegate `ProcessForScore`) 1.0 true))
  (set `self.TimerHandle` _returnvalue))

(event `ProcessForScore`
  (if (> (`KismetMathLibrary.VSize` (- (`SceneComponent.K2_GetComponentLocation` (`self.StaticMesh`)) (`self.StartingLocation`))) (`self.ScoreDistanceThreshold`))
    (`GameplayStatics.PlaySound2D` "/Game/Terror/Audio/A_BuildingCollapse.A_BuildingCollapse" 1.0 1.0 0.0 null null)
    (`/Game/Terror/Core/BP_GameMode.AddScore` (cast `/Game/Terror/Core/BP_GameMode` (`GameplayStatics.GetGameMode`) :!pure true) (`self.Points`))
    (`KismetSystemLibrary.K2_ClearAndInvalidateTimerHandle` (`self.TimerHandle`))))

(fn `UserConstructionScript`
  (`PrimitiveComponent.SetMaterial` (`self.StaticMesh`) 0 (`self.MaterialInstance`))
  (set `self.StartingLocation` (`SceneComponent.K2_GetComponentLocation` (`self.StaticMesh`))))