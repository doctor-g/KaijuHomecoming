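; BP_GameMode is the game mode for the Terror game, running a countdown timer and keeping score.
; StartGame sets the state to Playing, and Tick then subtracts delta time from the remaining seconds only in that state.
; When time runs out, the state switches to End and the game-end call fires.
; AddScore adds points to the running score without checking the state.
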(event `self.ReceiveTick`
  (params (DeltaSeconds :type "Float (single-precision)"))
  (switch `/Game/Terror/Core/EGameModeState` (`self.State`)
    (:`NewEnumerator1`
      (bind _output_get (set `self.SecondsRemaining` (- (`self.SecondsRemaining`) DeltaSeconds)))
      (if (<= _output_get 0.0)
        (set `self.State` "NewEnumerator2")
        (`self.OnGameEnd`)))))

(event `StartGame`
  (set `self.State` "NewEnumerator1"))

(event `AddScore`
  (params (Points :type Integer))
  (set `self.Score` (+ Points (`self.Score`))))

(fn `UserConstructionScript`)