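; BP_Column is a building column that awards points once it is knocked far enough from its original position.
; The construction script records the Cylinder's world location as the starting point.
; From BeginPlay, a looping one-second timer compares the current location against it.
; Past the distance threshold, it plays a collapse sound, adds its Points to BP_GameMode and clears the timer, so it scores only once.
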(event `self.ReceiveBeginPlay`
  (bind _returnvalue (`KismetSystemLibrary.K2_SetTimerDelegate` (delegate `ProcessForScore`) 1.0 true))
  (set `self.TimerHandle` _returnvalue))

(event `ProcessForScore`
  (if (> (`KismetMathLibrary.VSize` (- (`self.InitialLocation`) (`SceneComponent.K2_GetComponentLocation` (`self.Cylinder`)))) (`self.ScoreDistanceThreshold`))
    (`GameplayStatics.PlaySound2D` "/Game/Terror/Audio/A_BuildingCollapse.A_BuildingCollapse" 1.0 1.0 0.0 null null)
    (`/Game/Terror/Core/BP_GameMode.AddScore` (cast `/Game/Terror/Core/BP_GameMode` (`GameplayStatics.GetGameMode`) :!pure true) (`self.Points`))
    (`KismetSystemLibrary.K2_ClearAndInvalidateTimerHandle` (`self.TimerHandle`))))

(fn `UserConstructionScript`
  (set `self.InitialLocation` (`SceneComponent.K2_GetComponentLocation` (`self.Cylinder`))))