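; Player Blueprint for the Kaiju game that charges and launches fireballs.
; StartFireball spawns a BP_Fireball, and Tick pins its mesh to the spawn point while it grows.
; LaunchFireball stops growth, enables physics, applies a velocity-change impulse along the actor's forward vector, clears the reference and plays a sound.
; A validity check on launch ignores a stray first mouse release from a different state.
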(event `self.ReceiveTick`
  (params (DeltaSeconds :type "Float (single-precision)"))
  ;[1 1 1] Keep the fireball in front of the player while it is growing
  (`/Engine/EditorBlueprintResources/StandardMacros.IsValid` (`self.Fireball`)
    (:`Is Valid`
      (if (not (`self.FireballLaunched`))
        (`SceneComponent.K2_SetWorldLocation` (`StaticMeshActor.StaticMeshComponent` (`self.Fireball`)) (`SceneComponent.K2_GetComponentLocation` (`self.FireballSpawnLocation`)) false true)))))

(event `StartFireball`
  ;[1 1 1] Create a fireball
  (set `self.FireballLaunched` false)
  (bind _returnvalue (`|SpawnActorFromClass` "/Game/Terror/Kaiju/BP_Fireball.BP_Fireball_C" (`SceneComponent.K2_GetComponentToWorld` (`self.FireballSpawnLocation`)) "Undefined" "OverrideRootScale" null null))
  (set `self.Fireball` _returnvalue))

(event `LaunchFireball`
  (bind _fireball (`self.Fireball`))
  (bind _staticmeshcomponent (`StaticMeshActor.StaticMeshComponent` _fireball))
  ;[1 1 1] Launch a fireball
  (`/Engine/EditorBlueprintResources/StandardMacros.IsValid` (`self.Fireball`) ; Watch out for first mouse release, which is coming from a different state.
    (:`Is Valid`
      (set `self.FireballLaunched` true)
      (`/Game/Terror/Kaiju/BP_Fireball.StopGrowing` _fireball)
      (`PrimitiveComponent.SetSimulatePhysics` _staticmeshcomponent true)
      (`PrimitiveComponent.AddImpulse` _staticmeshcomponent (* (`self.GetActorForwardVector`) (`self.FireballVelocity`)) "None" true)
      (set `self.Fireball` null)
      (`GameplayStatics.PlaySound2D` "/Game/Terror/Audio/A_Fireball.A_Fireball" 1.0 1.0 0.0 null null))))

(fn `UserConstructionScript`)