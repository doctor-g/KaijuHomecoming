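; BP_PlayerController is the player controller that runs UI and input across the game's Splash, Playing and End states.
; It swaps splash, time-remaining and end widgets, starting the game through BP_GameMode and listening for its game-end event.
; A SwitchOnGameModeState macro gates fireball charge/launch and start/restart input by state, while look axes feed the controlled pawn.
; On game end, any charging fireball is launched, and restarting reloads DefaultMap.
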(event `self.ReceiveBeginPlay`
  (`WidgetBlueprintLibrary.SetInputMode_GameOnly` self)
  (bind _returnvalue (`|CreateWidget` "/Game/Terror/UI/Widget_Splash.Widget_Splash_C" self))
  (bind _output_get (set `self.SplashUI` _returnvalue))
  (`UserWidget.AddToViewport` _output_get 0)
  (add `/Game/Terror/Core/BP_GameMode.OnGameEnd` (cast `/Game/Terror/Core/BP_GameMode` (`GameplayStatics.GetGameMode`) :!pure true) (delegate `OnGameEnd`)))

(event `OnGameEnd`
  (`Widget.RemoveFromParent` (`self.PlayingUI`))
  (bind _returnvalue (`|CreateWidget` "/Game/Terror/UI/Widget_End.Widget_End_C" self))
  (`UserWidget.AddToViewport` _returnvalue 0)
  (`/Game/Terror/Kaiju/BP_Player.LaunchFireball` (cast `/Game/Terror/Kaiju/BP_Player` (`self.K2_GetPawn`) :!pure true)) ; If they were charging it up, let it go.
)

(event `InputAction|Quit`
  (params (Key :type "Key Structure"))
  (:`Pressed`
    (`KismetSystemLibrary.QuitGame` null "Quit")))

(event `InputAxis|Turn` :overrideparent false
  (params (AxisValue :type "Float (single-precision)"))
  (`Pawn.AddControllerYawInput` (`self.K2_GetPawn`) AxisValue))

(event `InputAxis|LookUp` :overrideparent false
  (params (AxisValue :type "Float (single-precision)"))
  (`Pawn.AddControllerPitchInput` (`self.K2_GetPawn`) AxisValue))

(event `InputAction|StartFireball`
  (params (Key :type "Key Structure"))
  (bind _asbp_player (cast `/Game/Terror/Kaiju/BP_Player` (`self.K2_GetPawn`) :!pure true))
  (:`Pressed`
    (`self.SwitchOnGameModeState`
      (:`Playing`
        (`/Game/Terror/Kaiju/BP_Player.StartFireball` _asbp_player))))
  (:`Released`
    (`self.SwitchOnGameModeState`
      (:`Playing`
        (`/Game/Terror/Kaiju/BP_Player.LaunchFireball` _asbp_player)))))

(event `InputAction|StartGame`
  (params (Key :type "Key Structure"))
  (:`Pressed`
    (`self.SwitchOnGameModeState`
      (:`Splash`
        (`/Game/Terror/Core/BP_GameMode.StartGame` (cast `/Game/Terror/Core/BP_GameMode` (`GameplayStatics.GetGameMode`) :!pure true))
        (`GameplayStatics.PlaySound2D` "/Game/Terror/Audio/A_Roar.A_Roar" 1.0 1.0 0.0 null null)
        (`Widget.RemoveFromParent` (`self.SplashUI`))
        (bind _returnvalue (`|CreateWidget` "/Game/Terror/UI/Widget_TimeRemaining.Widget_TimeRemaining_C" self))
        (bind _output_get (set `self.PlayingUI` _returnvalue))
        (`UserWidget.AddToViewport` _output_get 0))
      (:`End`
        (`GameplayStatics.OpenLevel` "DefaultMap")))))

(fn `GetGameModeState`
  (returns (State :type "/Game/Terror/Core/EGameModeState Enum"))
  (return (`/Game/Terror/Core/BP_GameMode.State` (cast `/Game/Terror/Core/BP_GameMode` (`GameplayStatics.GetGameMode`) :!pure true))))

(fn `UserConstructionScript`)