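; BP_Fireball is a fireball actor, filed with the Kaiju assets, that spins and grows over time.
; BeginPlay gives its RotatingMovement component a scaled-down random rotation rate.
; While Growing is set, Tick enlarges the actor by a fixed factor each frame until MaximumGrowthTime, overriding mesh mass in proportion to scale vector length.
; StopGrowing clears the flag to end growth early, and per-frame scaling makes final size frame-rate dependent.
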(event `self.ReceiveBeginPlay`
  ;[1 1 1] Add a random spin to the fireball
  (set `RotatingMovementComponent.RotationRate` (* (`KismetMathLibrary.RandomRotator` false) 0.2) (`self.RotatingMovement`)))

(event `self.ReceiveTick`
  (params (DeltaSeconds :type "Float (single-precision)"))
  (bind _returnvalue (* (`self.GetActorScale3D`) 1.01))
  (if (`self.Growing`)
    (bind _output_get (set `self.ElapsedGrowthTime` (+ DeltaSeconds (`self.ElapsedGrowthTime`))))
    (if (<= _output_get (`self.MaximumGrowthTime`))
      (`self.SetActorScale3D` _returnvalue)
      (`PrimitiveComponent.SetMassOverrideInKg` (`self.StaticMeshComponent`) "None" (* (`KismetMathLibrary.VSize` _returnvalue) 200.0) true))))

(event `StopGrowing`
  (set `self.Growing` false))

(fn `UserConstructionScript`)